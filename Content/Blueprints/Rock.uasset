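; Rock hazard actor that can hit Hugo, apparently inheriting most of its behavior from a parent class.
; On overlap it checks the other actor's name: a Hugo hit fires the hit-by-rock dispatcher with its value and plays a sound, otherwise it checks for the respawn trigger.
; Every overlap then resets position, scale and value, and pauses movement for a short random delay.
; Tick defers to the parent; ApplyEffect is empty.
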(event `self.ReceiveActorBeginOverlap`
  (params (OtherActor :type "Actor Object Reference"))
  (bind _returnvalue (`KismetSystemLibrary.GetObjectName` OtherActor))
  ;[1 1 1] Check if rock hit Hugo
  (bind _hitresult (`self.CheckHugoHit` _returnvalue))
  (if _hitresult
    ;[1 1 1] Play sound when Hugo is hit by rock
    (`self.HitByRockEventDispacher` (`self.Value`))
    (`GameplayStatics.PlaySound2D` "/Game/Sounds/RockHit_SC.RockHit_SC" 1.0 1.0 0.1 null null)
    (else
      ;[1 1 1] If not, check if rock hit Respawn trigger
      (`self.CheckRespawnHit` _returnvalue)))
  ;[1 1 1] Reset rock scale and value
  (`self.ResetPosition`)
  (`self.ResetScaleAndValue`)
  ;[1 1 1] Add delay to Rock moving again
  (set `self.Permit to Move` false)
  (`KismetSystemLibrary.Delay` (`KismetMathLibrary.RandomFloatInRange` 1.0 2.0))
  (set `self.Permit to Move` true))

(event `self.ReceiveTick`
  (params (DeltaSeconds :type "Float (single-precision)"))
  (`parent.ReceiveTick` 0.0))

(fn `ApplyEffect`)

(fn `UserConstructionScript`)